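; Interior door Blueprint that swings open and closed through a fingerprint scanner.
; On BeginPlay it caches the AllVar actors, and its scanner event proceeds only if the first one's FingerprintChecked flag is set.
; An accepted scan updates the scanner material and text, then a FlipFlop alternates open and close timelines that drive the door's yaw.
; The scanner material and text change again when closing finishes.
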(event `self.ReceiveBeginPlay`
  (bind _outactors (`GameplayStatics.GetAllActorsOfClass` "/Game/Blueprints/AllVar.AllVar_C")))

(event `OpenDoorWithFingerPrintScanner`
  (bind _door (`self.Door`))
  (if (`/Game/Blueprints/AllVar.FingerprintChecked` (`|GetArrayItem` (stale `self.ReceiveBeginPlay` _outactors)))
    (`PrimitiveComponent.SetMaterial` (`self.FingerPrint`) 0 "/Game/Blueprints/M2.M2")
    (`Text3DComponent.SetText` (`self.Finger Print Text`) (`self.Value1`))
    (`/Engine/EditorBlueprintResources/StandardMacros.FlipFlop`
      (:`A`
        (bind (_direction _doorfloat) (`Timeline|OpenDoorTimeLine` :!via `PlayFromStart`)
          (:`Update`
            (`SceneComponent.K2_SetRelativeRotation` _door (`KismetMathLibrary.MakeRotator` 0.0 0.0 (`KismetMathLibrary.Lerp` 180.0 90.0 _doorfloat)) false false))))
      (:`B`
        (bind (_direction_2 _closefloat) (`Timeline|CloseDoorTimeLine` :!via `PlayFromStart`)
          (:`Update`
            (`SceneComponent.K2_SetRelativeRotation` _door (`KismetMathLibrary.MakeRotator` 0.0 0.0 (`KismetMathLibrary.Lerp` 180.0 90.0 _closefloat)) false false))
          (:`Finished`
            (`PrimitiveComponent.SetMaterial` (`self.FingerPrint`) 0 "/Game/Blueprints/M1.M1")
            (`Text3DComponent.SetText` (`self.Finger Print Text`) (`self.Value2`))))))))

(fn `UserConstructionScript`)