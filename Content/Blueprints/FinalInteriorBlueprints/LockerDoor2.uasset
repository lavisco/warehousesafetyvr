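; LockerDoor2 is an interactable locker door that swings back and forth with steel door sound effects.
; Each Interact call alternates through a FlipFlop between playing and reversing a Timeline, which lerps the door's relative yaw across a quarter turn.
; Each direction stops one sound component and plays the other, with the swap on the reverse swing slightly delayed.
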(event `/Game/VRTemplate/Blueprints/Interact.Interact`
  (`/Engine/EditorBlueprintResources/StandardMacros.FlipFlop`
    (:`A`
      (`AudioComponent.Stop` (`self.ES_Steel_Door_-_SFX_Producer`))
      (`AudioComponent.Play` (`self.ES_Steel_Door_31_-_SFX_Producer`) 0.0)
      (bind (_direction _doorfloat) (`Timeline|Timeline` :!label _label)
        (:`Update`
          (`SceneComponent.K2_SetRelativeRotation` (`self.Door`) (`KismetMathLibrary.MakeRotator` 0.0 0.0 (`KismetMathLibrary.Lerp` -90.0 0.0 _doorfloat)) false false))))
    (:`B`
      (`|ExecutionSequence`
        (:`then_0`
          (goto _label :!via `Reverse`))
        (:`then_1`
          (`KismetSystemLibrary.Delay` 0.2)
          (`AudioComponent.Stop` (`self.ES_Steel_Door_31_-_SFX_Producer`))
          (`AudioComponent.Play` (`self.ES_Steel_Door_-_SFX_Producer`) 0.0))))))

(fn `UserConstructionScript`)