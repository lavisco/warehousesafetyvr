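; BPDoor is a door with a fingerprint scanner that swings open on a custom event and closes itself automatically.
; OpenDoorWithFingerPrintScanner swaps the scanner's material and text, then plays a timeline that lerps the door's yaw through a quarter turn.
; After a short delay, a second timeline drives the same lerp to close the door, then switches the scanner's material and text again.
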(event `OpenDoorWithFingerPrintScanner`
  (bind _door (`self.Door`))
  (`PrimitiveComponent.SetMaterial` (`self.FingerPrint`) 0 "/Game/Blueprints/M2.M2")
  (`Text3DComponent.SetText` (`self.Finger Print Text`) (`self.Value1`))
  (bind (_direction _doorfloat) (`Timeline|OpenDoorTimeLine` :!via `PlayFromStart`)
    (:`Update`
      (`SceneComponent.K2_SetRelativeRotation` _door (`KismetMathLibrary.MakeRotator` 0.0 0.0 (`KismetMathLibrary.Lerp` 0.0 -90.0 _doorfloat)) false false))
    (:`Finished`
      (`KismetSystemLibrary.Delay` 3.0)
      (bind (_direction_2 _closefloat) (`Timeline|CloseDoorTimeLine` :!via `PlayFromStart`)
        (:`Update`
          (`SceneComponent.K2_SetRelativeRotation` _door (`KismetMathLibrary.MakeRotator` 0.0 0.0 (`KismetMathLibrary.Lerp` 0.0 -90.0 _closefloat)) false false))
        (:`Finished`
          (`PrimitiveComponent.SetMaterial` (`self.FingerPrint`) 0 "/Game/Blueprints/M1.M1")
          (`Text3DComponent.SetText` (`self.Finger Print Text`) (`self.Value2`)))))))

(fn `UserConstructionScript`)