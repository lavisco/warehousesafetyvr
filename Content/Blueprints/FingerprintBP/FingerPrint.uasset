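; Fingerprint scanner Blueprint that responds to an interaction event with screen, text and audio feedback.
; FingerPrintInteract swaps the screen material and text, plays a keypad sound, then a sci-fi voice clip after a short delay.
; It finds the first AllVar actor via GetAllActorsOfClass and sets its FingerprintChecked flag.
; A few seconds later, it switches the screen to another material and text, with the flag left set.
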(event `/Game/Blueprints/FingerprintBP/FingerPrint_Interact.FingerPrintInteract`
  (`PrimitiveComponent.SetMaterial` (`self.Screen`) 0 "/Game/Blueprints/M2.M2")
  (`Text3DComponent.SetText` (`self.FingerPrintText`) (`self.Value1`))
  (`AudioComponent.Play` (`self.ES_Alarm_System_Keypad_1_-_SFX_Producer`) 0.0)
  (`KismetSystemLibrary.Delay` 0.4)
  (`AudioComponent.Play` (`self.ES_Sci_Fi_Voice_Clip_668_-_SFX_Producer`) 0.0)
  (bind _outactors (`GameplayStatics.GetAllActorsOfClass` "/Game/Blueprints/AllVar.AllVar_C"))
  (set `/Game/Blueprints/AllVar.FingerprintChecked` true (`|GetArrayItem` _outactors))
  (`KismetSystemLibrary.Delay` 5.0)
  (`PrimitiveComponent.SetMaterial` (`self.Screen`) 0 "/Game/Blueprints/M1.M1")
  (`Text3DComponent.SetText` (`self.FingerPrintText`) (`self.Value2`)))

(fn `UserConstructionScript`)